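; Blueprint function library with lookup helpers for card data tables.
; GetRandomRowFromDataTable returns a uniformly random row from the given table, printing a message when the table is empty.
; GetIconForCardType scans table rows for the first whose CardType matches by enum string and returns its Icon, calling ExportTexture2D before returning when none match.
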(fn GetRandomRowfromDataTable
  (params (Data_Table :type Data%20Table%20Object%20Reference))
  (bind _output_get (LocalVariables|Set_dataTable Data_Table))
  (bind _outrownames (DataTable|GetDataTableRowNames _output_get))
  (if (> (Utilities|Array|Length _outrownames) 0)
    (bind _returnvalue (Utilities|GetDataTableRow (LocalVariables|Get_dataTable) (Utilities|Array|Get(acopy) _outrownames (Math|Random|RandomIntegerinRange 0 (- (Utilities|Array|Length _outrownames) 1))))
      (:then
        _))
    (else
      (Development|PrintString 0 "No data in Cards data table")))
  (return _returnvalue))

(fn GetIconforCardType
  (params (Card%20Type :type ECardType%20Enum :default "Weapon"))
  (bind _outrownames (DataTable|GetDataTableRowNames (LocalVariables|Get_dataTable)))
  (for _array_element _outrownames
    (bind _returnvalue (Utilities|GetDataTableRow (LocalVariables|Get_dataTable) _array_element)
      (:then
        (if (Utilities|Enum|Equal(Enum) (Utilities|String|EnumtoString (.Card_Type (Utilities|Struct|BreakCard_Type_To_Icon_Struct _returnvalue))) (Utilities|String|EnumtoString Card%20Type))
          (return (.Icon (Utilities|Struct|BreakCard_Type_To_Icon_Struct _returnvalue)))))))
  (Class|KismetRenderingLibrary|ExportTexture2D)
  (return (.Icon (Utilities|Struct|BreakCard_Type_To_Icon_Struct _returnvalue))))